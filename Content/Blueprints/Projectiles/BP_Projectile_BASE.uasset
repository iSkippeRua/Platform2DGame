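; Base projectile actor that damages action characters of an opposing faction and destroys itself on impact.
; A blocking hit on its Sphere component spawns the hit effect and destroys the projectile without dealing damage.
; An overlap applies projectile damage only to characters of a different faction, then spawns the effect and destroys itself; other overlaps are ignored.
; PlayHitEffects spawns the shoot-hit VFX actor at the projectile's location and rotation.
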(event `self.Sphere.OnComponentHit`
  (params (HitComponent :type "PrimitiveComponent Object Reference") (OtherActor :type "Actor Object Reference") (OtherComp :type "PrimitiveComponent Object Reference") (NormalImpulse :type "Vector Structure") (Hit :type "HitResult Structure (by ref)"))
  (`self.PlayHitEffects`)
  (`self.K2_DestroyActor`))

(event `self.Sphere.OnComponentBeginOverlap`
  (params (OverlappedComponent :type "PrimitiveComponent Object Reference") (OtherActor :type "Actor Object Reference") (OtherComp :type "PrimitiveComponent Object Reference") (OtherBodyIndex :type Integer) (bFromSweep :type Boolean) (SweepResult :type "HitResult Structure (by ref)"))
  (bind _asbp_action_character_base (cast `/Game/Blueprints/Characters/BP_ActionCharacter_BASE` OtherActor))
  (if (`|EnumInequality` (`/Game/Blueprints/Characters/BP_ActionCharacter_BASE.Faction` _asbp_action_character_base) (`self.Faction`))
    (`GameplayStatics.ApplyDamage` _asbp_action_character_base (`self.ProjectileDamage`))
    (`self.PlayHitEffects`)
    (`self.K2_DestroyActor`)))

(fn `PlayHitEffects`
  (`|SpawnActorFromClass` "/Game/Blueprints/VFX/BP_VFX_ShootHit.BP_VFX_ShootHit_C" (`KismetMathLibrary.MakeTransform` (`self.K2_GetActorLocation`) (`self.K2_GetActorRotation`)) "AlwaysSpawn" "MultiplyWithRoot" null null))

(fn `UserConstructionScript`)